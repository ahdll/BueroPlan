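; BP_Calc is an area readout actor that displays the footprint of its scaled Scene component in square meters and pyeong.
; The construction script multiplies Scene's world X and Y scale, treating one scale unit as a meter, and divides by 3.305785 for the pyeong figure.
; It writes both values to the Data text and inverse-scales that component to offset stretching.
; The event graph holds only disabled placeholder events.
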(fn `UserConstructionScript`
  (bind _returnvalue (`SceneComponent.K2_GetComponentScale` (`self.Scene`)))
  (bind _returnvalue_2 (* (.x _returnvalue) (.y _returnvalue)))
  (`SceneComponent.SetRelativeScale3D` (`self.data`) (/ (1.0 1.0 1.0) _returnvalue))
  (`TextRenderComponent.K2_SetText` (`self.data`) (`KismetTextLibrary.Conv_StringToText` (`KismetStringLibrary.Concat_StrStr` "SquareMeter : " (`KismetStringLibrary.Conv_DoubleToString` _returnvalue_2) " \nPy : " (`KismetStringLibrary.Conv_DoubleToString` (/ _returnvalue_2 3.305785))))))